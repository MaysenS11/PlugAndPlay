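; Conveyor segment actor that continuously travels along the spline of a referenced track.
; On BeginPlay it converts its world position into a fraction of spline length, using that as the timeline's start time and Acceleration as its play rate.
; Timeline updates set location and rotation along the spline; after the first partial lap, it replays from the start.
; The Acceleration-from-Duration calculation is unconnected, and CalculateSpeed is empty.
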(event Custom|GetStartLocation
  (bind _track (Variables|Default|GetTrack))
  (bind _trackspine (Variables|/Game/PCG/BP_Track.BP_Track_C|GetTrackSpine _track))
  ;[0.1204 0.15 0.04216 0.5] SetStartLocationOnSpline
  (Utilities|IsValid _trackspine
    (:Is%20Valid
      (bind _output_get (Variables|Default|SetTrackSpline _trackspine))
      (Variables|Default|SetlocationPercentage (* 0.01 (* (Math|Float|SafeDivide (Class|SplineComponent|GetDistanceAlongSplineatLocation _output_get (Transformation|GetActorLocation) "World") (Spline|GetSplineLength (Variables|Default|GetTrackSpline))) 1e+02))))))

(event Custom|CalculateSpeed
  ;[0.15 0.15 0.15 0.5] CalculateSpeed
)

(event Custom|ConveyourTrack
  ;[0.15 0.08275 0.1474 0.5] Timeline
  (if (Variables|Default|GetFirstRound)
    (bind _distance (Timeline|ConveyourTimeline Play)
      (:Update
        (CallFunction|MoveSegment _distance))
      (:Finished
        (Variables|Default|SetFirstRound false)
        (CallFunction|ConveyourTrack)))
    (else
      (Timeline|ConveyourTimeline PlayFromStart))))

(event Custom|MoveSegment
  (params (Distance :type Float%20%28double-precision%29))
  (bind _trackspline (Variables|Default|GetTrackSpline))
  (bind _returnvalue (Spline|GetSplineLength _trackspline))
  ;[0.04419 0.15 0.1449 0.5] Move&RotateSegment
  (Utilities|IsValid _trackspline
    (:Is%20Valid
      (Variables|Default|SetLocationOnSpline (Math|Float|Clamp(Float) (* Distance _returnvalue) 0.0 _returnvalue))
      (Transformation|SetActorLocation (Spline|GetLocationatDistanceAlongSpline (Variables|Default|GetTrackSpline) (Variables|Default|GetLocationOnSpline) "World") false false)
      (Transformation|SetActorRotation (Spline|GetRotationatDistanceAlongSpline (Variables|Default|GetTrackSpline) (Variables|Default|GetLocationOnSpline) "Local")))))

(event EventBeginPlay
  ;[0 0.07812 0.0197 0.5] BeginPlay
  (CallFunction|GetStartLocation)
  (Components|Timeline|SetNewTime (Variables|Default|GetConveyourTimeline) (Variables|Default|GetlocationPercentage))
  (Components|Timeline|SetPlayRate (Variables|Default|GetConveyourTimeline) (Variables|Default|GetAcceleration))
  (CallFunction|ConveyourTrack))

(fn ConstructionScript)