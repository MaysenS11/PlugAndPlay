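; CylinderGrav is an interactable gravity zone built around an axis running between its Start and End components.
; While the player overlaps its Box, it registers itself as the player's CylinderGrav and sets HasGravity, clearing both on exit.
; GravDirection projects a given location onto the Start-End segment, clamped to its ends, and returns that closest axis point rather than a direction vector.
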(event `self.Box.OnComponentBeginOverlap`
  (params (OverlappedComponent :type "PrimitiveComponent Object Reference") (OtherActor :type "Actor Object Reference") (OtherComp :type "PrimitiveComponent Object Reference") (OtherBodyIndex :type Integer) (bFromSweep :type Boolean) (SweepResult :type "HitResult Structure (by ref)"))
  (bind _asplayer (cast `/Game/Blueprints/player` OtherActor))
  (set `/Game/Blueprints/player.CylinderGrav` self _asplayer)
  (set `/Game/Blueprints/player.hasGravity` true _asplayer))

(event `self.Box.OnComponentEndOverlap`
  (params (OverlappedComponent :type "PrimitiveComponent Object Reference") (OtherActor :type "Actor Object Reference") (OtherComp :type "PrimitiveComponent Object Reference") (OtherBodyIndex :type Integer))
  (bind _asplayer (cast `/Game/Blueprints/player` OtherActor))
  (set `/Game/Blueprints/player.CylinderGrav` null _asplayer)
  (set `/Game/Blueprints/player.hasGravity` false _asplayer))

(fn `GravDirection`
  (params (ActorsLocation :type "Vector Structure"))
  (returns (Direction :type "Vector Structure"))
  (locals (Heading :type "Vector Structure") (Magnitude :type "Float (double-precision)" :default 0.0) (`Actor Location` :type "Vector Structure") (Lhs :type "Vector Structure") (DotProdukt :type "Float (double-precision)" :default 0.0))
  (bind _returnvalue (- (`SceneComponent.K2_GetComponentLocation` (`self.end`)) (`SceneComponent.K2_GetComponentLocation` (`self.start`))))
  (set `local.Actor Location` ActorsLocation)
  (set `local.Magnitude` (`KismetMathLibrary.VSize` _returnvalue))
  (set `local.Heading` (`KismetMathLibrary.Normal` _returnvalue))
  (bind _output_get (set `local.Lhs` (- (`local.Actor Location`) (`SceneComponent.K2_GetComponentLocation` (`self.start`))))) ; LeftHandSide
  (bind _output_get_2 (set `local.DotProdukt` (`KismetMathLibrary.Dot_VectorVector` _output_get (`local.Heading`))))
  (return (+ (`SceneComponent.K2_GetComponentLocation` (`self.start`)) (* (`local.Heading`) (`KismetMathLibrary.FClamp` _output_get_2 0.0 (`local.Magnitude`))))))

(fn `UserConstructionScript`)