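; Interactable lever that toggles a linked Level Sequence between forward and reverse playback.
; Each Interact flips the LeverOff flag, plays or reverses the sequence, and runs a Timeline that swings the handle between two yaw angles to match.
; InRange and LeaveRange events show and hide a TextRender prompt.
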(event `/Game/Blueprints/interfaces/interactable.interact`
  (if (`self.leverOff`)
    (set `self.leverOff` false)
    (`MovieSceneSequencePlayer.Play` (`LevelSequenceActor.SequencePlayer` (`self.levelSequence`)))
    (bind (_direction _newtrack_0) (`Timeline|Timeline` :!label _label)
      (:`Update`
        (`SceneComponent.K2_SetRelativeRotation` (`self.handle`) (`KismetMathLibrary.RLerp` (struct :`Pitch` -50.0) (struct :`Pitch` 50.0) _newtrack_0) false false)))
    (else
      (set `self.leverOff` true)
      (`MovieSceneSequencePlayer.PlayReverse` (`LevelSequenceActor.SequencePlayer` (`self.levelSequence`)))
      (goto _label :!via `Reverse`))))

(event `/Game/Blueprints/interfaces/interactable.inRange`
  (`SceneComponent.SetHiddenInGame` (`self.TextRender`) false false))

(event `/Game/Blueprints/interfaces/interactable.leaveRange`
  (`SceneComponent.SetHiddenInGame` (`self.TextRender`) true false))

(fn `UserConstructionScript`)