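; BP_PentalLights is a movable actor, apparently a hanging light, that swings endlessly like a pendulum around its roll axis from BeginPlay.
; A timeline, with play rate set from Duration, scales the Rotation amplitude into a clamped roll while keeping current pitch and yaw.
; Each finish alternates the timeline between Play and Reverse, and a FlipFlop switches swing side whenever the roll is not at maximum.
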(event `self.ReceiveBeginPlay`
  ;[0.7656 0.7656 0.7656 0.5] BeginPlay
  (`TimelineComponent.SetPlayRate` (`self.PendalTimeline`) (`self.Duration`))
  (`self.PendalTime`))

(event `PendalTime`
  ;[0.15 0.06492 0.1274 0.5] PendalTimeline
  (if (`self.TimelineForward`)
    (bind (_direction _pendaltime) (`Timeline|PendalTimeline` :!label _label)
      (:`Update`
        (if (`self.MovementForward`)
          (`self.RotateFrorward` _pendaltime)
          (else
            (`self.RotateBack` _pendaltime))))
      (:`Finished`
        (bind _isa (`/Engine/EditorBlueprintResources/StandardMacros.FlipFlop`)
          (:`A`
            _)
          (:`B`
            _))
        (set `self.TimelineForward` (not _isa))
        (`self.ChangeDirections`)))
    (else
      (goto _label :!via `Reverse`))))

(event `ChangeDirections`
  ;[0.08386 0.06753 0.15 0.5] ChangeDirection
  (if (== (`self.Rotation`) (`KismetMathLibrary.Abs` (`self.ActiveRotation`)))
    (set `self.MaxReached` true)
    (else
      ;;[0.15 0.1109 0.04422 0.5] change direction
      (set `self.MaxReached` false)
      (bind _isa (`/Engine/EditorBlueprintResources/StandardMacros.FlipFlop`)
        (:`A`
          _)
        (:`B`
          _))
      (set `self.MovementForward` _isa)))
  (`self.PendalTime`))

(event `RotateFrorward`
  (params (PendalTime :type "Float (double-precision)"))
  (bind (_returnvalue_pitch _returnvalue_yaw) (`self.Y&Z_Rotation`))
  (bind _rotation (`self.Rotation`))
  ;[0.04777 0.1875 0.07878 0.1478] Rotation
  ;;[0.162 0.3185 0.1981 0.502] Forward
  (bind _output_get (set `self.ActiveRotation` (`KismetMathLibrary.FClamp` (* PendalTime _rotation) 0.0 _rotation)))
  (`self.K2_SetActorRotation` (`KismetMathLibrary.MakeRotator` _output_get _returnvalue_pitch _returnvalue_yaw)))

(event `RotateBack`
  (params (PendalTime :type "Float (double-precision)"))
  (bind (_returnvalue_pitch _returnvalue_yaw) (`self.Y&Z_Rotation`))
  (bind _returnvalue (* -1.0 (`self.Rotation`)))
  ;[0.04777 0.1875 0.07878 0.1478] Rotation
  ;;[0.02914 0.05729 0.03562 0.7739] Backwards
  (bind _output_get (set `self.ActiveRotation` (`KismetMathLibrary.FClamp` (* PendalTime _returnvalue) _returnvalue)))
  (`self.K2_SetActorRotation` (`KismetMathLibrary.MakeRotator` _output_get _returnvalue_pitch _returnvalue_yaw)))

(fn `UserConstructionScript`)