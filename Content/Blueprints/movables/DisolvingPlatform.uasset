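; A platform that shrinks away after the player touches it, then respawns.
; Box overlap starts a short delay, then a timeline alpha scales the actor down from its default, dropping collision near the end and hiding it on finish.
; Respawn restores scale, visibility and collision after a delay.
; Leaving the box also schedules a respawn, stopping the timeline if the timer value is still high enough.
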(event `self.Box.OnComponentBeginOverlap`
  (params (OverlappedComponent :type "PrimitiveComponent Object Reference") (OtherActor :type "Actor Object Reference") (OtherComp :type "PrimitiveComponent Object Reference") (OtherBodyIndex :type Integer) (bFromSweep :type Boolean) (SweepResult :type "HitResult Structure (by ref)"))
  (cast `/Game/Blueprints/player` OtherActor)
  (`self.DisolvePlatform`))

(event `DisolvePlatform`
  (bind (_defscale_location _defscale_rotation _defscale_scale) (`KismetMathLibrary.BreakTransform` (`self.DefScale`)))
  (bind (_defscale_location_2 _defscale_rotation_2 _defscale_scale_2) (`KismetMathLibrary.BreakTransform` (`self.DefScale`)))
  (`KismetSystemLibrary.Delay` 0.3)
  (if (`KismetMathLibrary.NotEqualExactly_VectorVector` (`self.GetActorScale3D`) _defscale_scale_2)
    (bind (_direction _alpha) (`Timeline|Timeline` :!label _label)
      (:`Update`
        (bind _output_get (set `self.PlatformTimer` _alpha))
        (`self.SetActorScale3D` (* _output_get _defscale_scale))
        (if (<= (`self.PlatformTimer`) 0.2)
          (`self.SetActorEnableCollision` false)))
      (:`Finished`
        (`self.SetActorHiddenInGame` true)
        (`self.RespawnPlatform`)))
    (else
      (goto _label :!via `PlayFromStart`))))

(event `self.Box.OnComponentEndOverlap`
  (params (OverlappedComponent :type "PrimitiveComponent Object Reference") (OtherActor :type "Actor Object Reference") (OtherComp :type "PrimitiveComponent Object Reference") (OtherBodyIndex :type Integer))
  (cast `/Game/Blueprints/player` OtherActor)
  (`|ExecutionSequence`
    (:`then_0`
      (if (>= (`self.PlatformTimer`) 0.5)
        (goto _label :!via `Stop`)
        (else
          _)))
    (:`then_1`
      _))
  (`self.RespawnPlatform`))

(event `RespawnPlatform`
  (bind (_defscale_location _defscale_rotation _defscale_scale) (`KismetMathLibrary.BreakTransform` (`self.DefScale`)))
  (`KismetSystemLibrary.Delay` 2.0)
  (`self.SetActorScale3D` _defscale_scale)
  (`self.SetActorHiddenInGame` false)
  (`self.SetActorEnableCollision` true))

(fn `UserConstructionScript`)