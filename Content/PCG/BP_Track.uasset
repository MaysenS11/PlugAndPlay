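; BP_Track is a spline-based track actor in the PCG folder, built around a TrackSpine spline.
; Its construction script only stores a self reference in Track, and BeginPlay does nothing.
; Unconnected construction nodes would read the start location and tangent and sample segment locations along the spline by width plus spacing, but they never run.
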(event EventBeginPlay)

(fn ConstructionScript
  (Variables|Default|SetTrack self))